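; Steering actor implementing arrival behaviour: moves forward along its local X axis, turns toward a target, slows and stops on approach.
; BeginPlay gathers all actors of the Target classes; each Tick interpolates rotation toward the lowest stored distance.
; Distances refresh only while ClosestTarget is set; threshold checks scale Velocity by distance or zero it, never restoring cruise speed.
; The construction script adds the configurable static mesh.
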(event EventBeginPlay
  ;[0 0.5598 1] Obtiene el target al que se dirigirá el objeto.
  (for _array_element (Variables|Arrival|GetTarget)
    (bind _outactors (Actor|GetAllActorsOfClass _array_element))
    (for _array_element_2 _outactors
      (Utilities|Array|Add (Variables|Default|GetArrivalTarget) _array_element_2))))

(event EventTick
  (params (DeltaSeconds :type Float%20%28single-precision%29))
  (Utilities|FlowControl|Sequence
    (:then_0
      ;[1 0 0] Hace que el objeto avance sobre el eje X (hace que avance).
      (Transformation|AddActorLocalOffset (Math|Vector|MakeVector (Variables|Arrival|GetVelocity) 0.0 0.0) false false))
    (:then_1
      ;[0 0.08456 1] El objeto se dirigirá hacia la posición de su Target.
      (Transformation|SetActorRotation (Math|Interpolation|RInterpTo (Transformation|GetActorRotation) (Math|Rotator|FindLookatRotation (Transformation|GetActorLocation) (Transformation|GetActorLocation (Utilities|Array|Get(acopy) (Variables|Default|GetArrivalTarget) (.IndexOfMinValue (Math|Float|MinOfFloatArray (Variables|Default|GetArrivalDistance)))))) (Utilities|Time|GetWorldDeltaSeconds) 5.0)))
    (:then_2
      (if (Variables|Arrival|GetClosestTarget)
        (for (_array_element _array_index) (Variables|Default|GetArrivalTarget)
          ;[0.04861 1 0] Guardar la distancia entre el objeto y su target.
          (Utilities|Array|SetArrayElem (Variables|Default|GetArrivalDistance) _array_index (Transformation|GetDistanceTo _array_element) true)
          ;[0.04655 1 0] Elegir una distancia mínima entre el objeto y su target.
          (if (> (Transformation|GetDistanceTo _array_element) (Variables|Arrival|GetDecelerationMinimumDistance)) ; Verifica si la distancia es mayor a las unidades especificadas, si esta es mayor entonces continua con su velocidad. Vuelve a verificar si la distancia es mayor a las unidades especificadas, si es así entonces se iniciará la segunda verificación.
            (Variables|Arrival|SetVelocity (Variables|Arrival|GetVelocity))
            (elif (> (Transformation|GetDistanceTo _array_element) (Variables|Arrival|GetStopMinimumDistance)) ; Al saber que la distancia es menor a las unidades especificadas, el objeto reducirá su velocidad hasta llegar al destino y detenerse.
              (Variables|Arrival|SetVelocity (/ (Transformation|GetDistanceTo _array_element) (Variables|Arrival|GetDecelerationIntensity)))
              (else
                (Variables|Arrival|SetVelocity 0.0)))))
        (else
          (if (> (Transformation|GetDistanceTo _array_element) (Variables|Arrival|GetDecelerationMinimumDistance)) ; Verifica si la distancia es mayor a las unidades especificadas, si esta es mayor entonces continua con su velocidad. Vuelve a verificar si la distancia es mayor a las unidades especificadas, si es así entonces se iniciará la segunda verificación.
            (Variables|Arrival|SetVelocity (Variables|Arrival|GetVelocity))
            (elif (> (Transformation|GetDistanceTo _array_element) (Variables|Arrival|GetStopMinimumDistance)) ; Al saber que la distancia es menor a las unidades especificadas, el objeto reducirá su velocidad hasta llegar al destino y detenerse.
              (Variables|Arrival|SetVelocity (/ (Transformation|GetDistanceTo _array_element) (Variables|Arrival|GetDecelerationIntensity)))
              (else
                (Variables|Arrival|SetVelocity 0.0)))))))))

(fn ConstructionScript
  ;[1 0 0.6777] Setear el mesh del objeto.
  (bind _returnvalue (AddComponent|AddStaticMeshComponent false (Math|Transform|MakeTransform "0, 0,-50.000000" "0, 0, 0" "1.000000,1.000000,1.000000")))
  (Components|StaticMesh|SetStaticMesh _returnvalue (Variables|Arrival|GetStaticMesh)))