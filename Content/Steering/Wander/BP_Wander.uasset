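; BP_Wander is a steering actor that wanders between random points in a box centered near the world origin, using a configurable static mesh added at construction.
; Each tick it moves along its local X by a per-frame Velocity and interpolates its rotation toward the destination.
; It picks a new point on arrival, or stops if Wait is set.
; While still travelling, a Delay also re-picks the destination every NewDirectionTime.
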(event EventBeginPlay
  ;[0.967 0 1] Elige un punto aleatorio para iniciar.
  (Variables|Default|SetNewDestination (Math|Random|RandomPointinBoundingBox "0, 0,50.000000" (Math|Vector|MakeVector (Variables|Wander|GetMaxBoxExtentX) (Variables|Wander|GetMaxBoxExtentY) (Variables|Wander|GetMaxBoxExtentZ)))))

(event EventTick
  (params (DeltaSeconds :type Float%20%28single-precision%29))
  (Utilities|FlowControl|Sequence
    (:then_0
      ;[1 0 0] Hace que el objeto avance sobre el eje X (hacia delante)
      (Transformation|AddActorLocalOffset (Math|Vector|MakeVector (Variables|Wander|GetVelocity) 0.0 0.0) false false))
    (:then_1
      ;[0 0.09893 1] El objeto rotará tomando como base su posición hacia una nueva posición.
      (Transformation|SetActorRotation (Math|Interpolation|RInterpTo (Transformation|GetActorRotation) (Math|Rotator|FindLookatRotation (Transformation|GetActorLocation) (Variables|Default|GetNewDestination)) (Utilities|Time|GetWorldDeltaSeconds) 5.0)))
    (:then_2
      ;[1 0.8337 0] Cada 2 segundos buscará una nueva posición hacia donde dirigirse.
      (if (<= (Math|Vector|Distance(Vector) (Transformation|GetActorLocation) (Variables|Default|GetNewDestination)) 1e+02)
        (if (Variables|Wander|GetWait)
          (Variables|Wander|SetVelocity 0.0)
          (else
            (Variables|Default|SetNewDestination (Math|Random|RandomPointinBoundingBox "0, 0,50.000000" (Math|Vector|MakeVector (Variables|Wander|GetMaxBoxExtentX) (Variables|Wander|GetMaxBoxExtentY) (Variables|Wander|GetMaxBoxExtentZ))) :!label _label)
            (Variables|Wander|SetVelocity 1e+01)))
        (else
          (Utilities|FlowControl|Delay (Variables|Wander|GetNewDirectionTime))
          (goto _label))))))

(fn ConstructionScript
  ;[1 0 0.8577] Setear el mesh del objeto.
  (bind _returnvalue (AddComponent|AddStaticMeshComponent false (Math|Transform|MakeTransform "0, 0,-50.000000" "0, 0, 0" "1.000000,1.000000,1.000000")))
  (Components|StaticMesh|SetStaticMesh _returnvalue (Variables|Wander|GetStaticMesh)))