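; Evade steering actor that moves forward every tick and turns away from targets gathered on BeginPlay from a list of classes.
; When within range of a point projected ahead of a target, it smoothly rotates away using look-at on negated positions.
; MultipleTarget checks every target; otherwise the check runs outside the loop on its index.
; Movement is not delta-time scaled; the construction script adds the configurable mesh.
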(event EventBeginPlay
  ;[0.4187 1 0.4793] Obtiene el target el cual evadirá.
  (for _array_element (Variables|Evade|GetEvadeTarget)
    (bind _outactors (Actor|GetAllActorsOfClass _array_element))
    (for _array_element_2 _outactors
      (Utilities|Array|Add (Variables|Default|GetTarget) _array_element_2))))

(event EventTick
  (params (DeltaSeconds :type Float%20%28single-precision%29))
  (Utilities|FlowControl|Sequence
    (:then_0
      ;[1 0 0.02893] Hace que el objeto avance sobre el eje X (hacia delante)
      (Transformation|AddActorLocalOffset (Math|Vector|MakeVector (Variables|Evade|GetVelocity) 0.0 0.0) false false))
    (:then_1
      (if (Variables|Evade|GetMultipleTarget)
        (for (_ _array_index) (Variables|Default|GetTarget)
          ;[0.9148 0 1] Define la distancia mínima entre el objeto y su target.
          (if (< (Math|Vector|Distance(Vector) (Transformation|GetActorLocation) (+ (Transformation|GetActorLocation (Utilities|Array|Get(acopy) (Variables|Default|GetTarget) _array_index)) (* (Transformation|GetActorForwardVector (Utilities|Array|Get(acopy) (Variables|Default|GetTarget) _array_index)) (Variables|Evade|GetTargetForwardDistance)))) (Variables|Evade|GetEffectMinimumDistance))
            ;[0 0.6423 1] El objeto girará a la ubicación opuesta a la que se encuentra su Target.
            (Transformation|SetActorRotation (Math|Interpolation|RInterpTo (Transformation|GetActorRotation) (Math|Rotator|FindLookatRotation (Math|Vector|NegateVector (Transformation|GetActorLocation)) (Math|Vector|NegateVector (+ (Transformation|GetActorLocation (Utilities|Array|Get(acopy) (Variables|Default|GetTarget) _array_index)) (* (Transformation|GetActorForwardVector (Utilities|Array|Get(acopy) (Variables|Default|GetTarget) _array_index)) (Variables|Evade|GetTargetForwardDistance))))) (Utilities|Time|GetWorldDeltaSeconds) 5.0))))
        (else
          (if (< (Math|Vector|Distance(Vector) (Transformation|GetActorLocation) (+ (Transformation|GetActorLocation (Utilities|Array|Get(acopy) (Variables|Default|GetTarget) _array_index)) (* (Transformation|GetActorForwardVector (Utilities|Array|Get(acopy) (Variables|Default|GetTarget) _array_index)) (Variables|Evade|GetTargetForwardDistance)))) (Variables|Evade|GetEffectMinimumDistance))
            (Transformation|SetActorRotation (Math|Interpolation|RInterpTo (Transformation|GetActorRotation) (Math|Rotator|FindLookatRotation (Math|Vector|NegateVector (Transformation|GetActorLocation)) (Math|Vector|NegateVector (+ (Transformation|GetActorLocation (Utilities|Array|Get(acopy) (Variables|Default|GetTarget) _array_index)) (* (Transformation|GetActorForwardVector (Utilities|Array|Get(acopy) (Variables|Default|GetTarget) _array_index)) (Variables|Evade|GetTargetForwardDistance))))) (Utilities|Time|GetWorldDeltaSeconds) 5.0))))))))

(fn ConstructionScript
  (bind _returnvalue (AddComponent|AddStaticMeshComponent false (Math|Transform|MakeTransform "0, 0,-50.000000" "0, 0, 0" "1.000000,1.000000,1.000000")))
  (Components|StaticMesh|SetStaticMesh _returnvalue (Variables|Evade|GetStaticMesh)))