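; BP_Flee is a steering-behavior actor whose physics-driven cone flees from the BP_FleeTarget found at BeginPlay.
; Each Tick, Flee builds a desired velocity away from the target and derives a steering force, scaled to MaxForce unless the difference is under one unit.
; The resulting velocity is rescaled to MaxVel and applied as linear velocity, then LookAtDirection orients the cone along it.
; Debug arrows show desired, steering and final vectors.
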(event Collision|EventActorBeginOverlap
  (params (OtherActor :type Actor%20Object%20Reference)))

(event EventBeginPlay
  (Variables|Default|SetCurrentVel "0.000000,0.000000,100.000000")
  (bind _returnvalue (Actor|GetActorOfClass "/Game/Steering/Flee/BP_FleeTarget.BP_FleeTarget_C"))
  (Variables|Default|SetTarget _returnvalue))

(event EventTick
  (params (DeltaSeconds :type Float%20%28single-precision%29))
  (CallFunction|Flee (Transformation|GetWorldLocation (Variables|/Game/Steering/Flee/BP_FleeTarget.BP_FleeTarget_C|GetCone (Variables|Default|GetTarget))) true)
  (Physics|SetPhysicsLinearVelocity (Variables|Default|GetCone) (Variables|Default|GetCurrentVel) false "None")
  (CallFunction|LookatDirection))

(fn ConstructionScript)

(fn Flee
  (params (Pos :type Vector) (Debug :type Boolean))
  (bind _cone (Variables|Default|GetCone))
  (bind _cone_2 (Variables|Default|GetCone))
  (bind _returnvalue (Transformation|GetWorldLocation _cone))
  (bind _returnvalue_2 (Transformation|GetWorldLocation _cone_2))
  (LocalVariables|Set_Debug Debug)
  (LocalVariables|SetTargetPos Pos)
  (Utilities|FlowControl|Sequence
    (:then_0
      ;[1 0 0.7929] SetDesireVel
      (Variables|Default|SetDesiredVel (* (Variables|Default|GetMaxVel) (Math|Vector|NegateVector (Math|Vector|Normalize (- (LocalVariables|GetTargetPos) (Transformation|GetWorldLocation (Variables|Default|GetCone))))))))
    (:then_1
      ;[0.1268 1 0] Debug DesiredVel
      (if (LocalVariables|Get_Debug)
        (Rendering|Debug|DrawDebugArrow _returnvalue_2 (+ _returnvalue_2 (Variables|Default|GetDesiredVel)) 1.0 "(R=1.000000,G=0.038740,B=0.000000,A=1.000000)" 0.0 0.0)))
    (:then_2
      ;[1 0 0.7462] SteeringVel
      (if (< (Math|Vector|VectorLength (- (Variables|Default|GetDesiredVel) (Variables|Default|GetCurrentVel))) (Math|Vector|VectorLength (Math|Vector|Normalize (- (Variables|Default|GetDesiredVel) (Variables|Default|GetCurrentVel)))))
        (Variables|Default|SetSteeringForce (- (Variables|Default|GetDesiredVel) (Variables|Default|GetCurrentVel)))
        (else
          (Variables|Default|SetSteeringForce (* (Math|Vector|Normalize (- (Variables|Default|GetDesiredVel) (Variables|Default|GetCurrentVel))) (Variables|Default|GetMaxForce))))))
    (:then_3
      ;[0.9713 1 0] Debug SteeringVel
      (if (LocalVariables|Get_Debug)
        (Rendering|Debug|DrawDebugArrow (+ (Transformation|GetWorldLocation (Variables|Default|GetCone)) (Variables|Default|GetCurrentVel)) (+ (+ (Transformation|GetWorldLocation (Variables|Default|GetCone)) (Variables|Default|GetCurrentVel)) (Variables|Default|GetSteeringForce)) 1.0 "(R=0.000000,G=0.101826,B=1.000000,A=1.000000)" 0.0 0.0)))
    (:then_4
      ;[1 0 0.8219] SetCurrentVelFinal
      (Variables|Default|SetCurrentVel (* (Math|Vector|Normalize (+ (Variables|Default|GetCurrentVel) (Variables|Default|GetSteeringForce))) (Variables|Default|GetMaxVel))))
    (:then_5
      ;[0.9713 1 0] Debug CurrentVelFinal
      (if (LocalVariables|Get_Debug)
        (Rendering|Debug|DrawDebugArrow _returnvalue (+ _returnvalue (Variables|Default|GetCurrentVel)) 1.0 "(R=0.000000,G=1.000000,B=0.046659,A=1.000000)" 0.0 0.0)))))

(fn LookatDirection
  (bind _cone (Variables|Default|GetCone))
  (bind _cone_2 (Variables|Default|GetCone))
  (bind _currentvel (Variables|Default|GetCurrentVel))
  (bind _returnvalue (Transformation|GetWorldLocation _cone))
  (bind _relativelocation (Variables|/Script/Engine.SceneComponent|GetRelativeLocation _cone_2))
  (bind _returnvalue_2 (+ _relativelocation _currentvel))
  (bind _returnvalue_3 (Math|Rotator|FindLookatRotation _returnvalue _returnvalue_2))
  (bind (_roll _pitch _yaw) (Math|Rotator|BreakRotator _returnvalue_3))
  (Transformation|SetWorldRotation (Variables|Default|GetCone) (Math|Rotator|MakeRotator _roll (+ _pitch -9e+01) _yaw) false false))