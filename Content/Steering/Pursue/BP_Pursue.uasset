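; Steering-behavior actor that pursues the nearest actor of its configured target classes, aiming at a point ahead of it.
; BeginPlay collects the targets; with ClosestTarget on, Tick records their distances and lowers or zeroes Velocity for any within deceleration or stop range.
; Each frame it moves along local X by Velocity, unscaled by delta time, and smoothly turns toward the nearest target's forward-offset position.
; The construction script adds its static mesh.
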(event EventBeginPlay
  ;[0.524 1 0.816] Setea el target que perseguirá.
  (for _array_element (Variables|Pursuit|GetTarget)
    (bind _outactors (Actor|GetAllActorsOfClass _array_element))
    (for _array_element_2 _outactors
      (Utilities|Array|Add (Variables|Default|GetPursuitTarget) _array_element_2))))

(event EventTick
  (params (DeltaSeconds :type Float%20%28single-precision%29))
  (bind _pursuittarget (Variables|Default|GetPursuitTarget))
  (bind _targetdistance (Variables|Default|GetTargetDistance))
  (bind _indexofminvalue (Math|Float|MinOfFloatArray _targetdistance))
  (bind _output (Utilities|Array|Get(acopy) _pursuittarget _indexofminvalue))
  (Utilities|FlowControl|Sequence
    (:then_0
      ;[1 0 0.05503] Hace que el objeto avance sobre el eje X (hacia delante)
      (Transformation|AddActorLocalOffset (Math|Vector|MakeVector (Variables|Pursuit|GetVelocity) 0.0 0.0) false false))
    (:then_1
      (if (Variables|Pursuit|GetClosestTarget)
        (for (_array_element _array_index) (Variables|Default|GetPursuitTarget)
          ;[0 1 0.2003] Guarda la distancia entre el objeto y el target.
          (Utilities|Array|SetArrayElem (Variables|Default|GetTargetDistance) _array_index (Transformation|GetDistanceTo _array_element) true)
          ;[0 1 0.15] Establece una distancia mínima entre el objeto y el target, al llegar a esta distancia mínima, el objeto disminuirá su velocidad (así no alcanzando al target)
          (if (> (Transformation|GetDistanceTo _array_element) (Variables|Default|GetDecelerationMinimumDistance)) ; Verifica si la distancia es mayor a las unidades especificadas, si esta es mayor entonces continua con su velocidad. Vuelve a verificar si la distancia es mayor a las unidades especificadas, si es así entonces se iniciará la segunda verificación.
            (Variables|Pursuit|SetVelocity (Variables|Pursuit|GetVelocity))
            (elif (> (Transformation|GetDistanceTo _array_element) (Variables|Default|GetStopMinimumDistance)) ; Al saber que la distancia es menor a las unidades especificadas, el objeto reducirá su velocidad hasta llegar al destino y detenerse.
              (Variables|Pursuit|SetVelocity (/ (Transformation|GetDistanceTo _array_element) (Variables|Default|GetDecelerationIntensity)))
              (else
                (Variables|Pursuit|SetVelocity 0.0)))))
        (else
          (if (> (Transformation|GetDistanceTo _array_element) (Variables|Default|GetDecelerationMinimumDistance)) ; Verifica si la distancia es mayor a las unidades especificadas, si esta es mayor entonces continua con su velocidad. Vuelve a verificar si la distancia es mayor a las unidades especificadas, si es así entonces se iniciará la segunda verificación.
            (Variables|Pursuit|SetVelocity (Variables|Pursuit|GetVelocity))
            (elif (> (Transformation|GetDistanceTo _array_element) (Variables|Default|GetStopMinimumDistance)) ; Al saber que la distancia es menor a las unidades especificadas, el objeto reducirá su velocidad hasta llegar al destino y detenerse.
              (Variables|Pursuit|SetVelocity (/ (Transformation|GetDistanceTo _array_element) (Variables|Default|GetDecelerationIntensity)))
              (else
                (Variables|Pursuit|SetVelocity 0.0)))))))
    (:then_2
      ;[0 0.1912 1] El objetivo tomará como su nuevo destino la ubicación del target.
      (Transformation|SetActorRotation (Math|Interpolation|RInterpTo (Transformation|GetActorRotation) (Math|Rotator|FindLookatRotation (Transformation|GetActorLocation) (+ (Transformation|GetActorLocation _output) (* (Transformation|GetActorForwardVector _output) (Variables|Pursuit|GetTargetForwardDistance)))) (Utilities|Time|GetWorldDeltaSeconds) 5.0)))))

(fn ConstructionScript
  (bind _returnvalue (AddComponent|AddStaticMeshComponent false (Math|Transform|MakeTransform "0, 0,-50.000000" "0, 0, 0" "1.000000,1.000000,1.000000")))
  (Components|StaticMesh|SetStaticMesh _returnvalue (Variables|Pursuit|GetStaticMesh)))