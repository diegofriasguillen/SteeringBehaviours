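; Wandering target actor for a pursue steering setup, roaming between random points in a box around a fixed center.
; Each tick it turns smoothly toward its destination with RInterpTo and steps forward by Velocity, unscaled by delta time.
; It picks a new destination on arrival or when a Delay started while travelling expires.
; If StopMoving is set, arrival zeroes its velocity instead.
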(event EventBeginPlay
  ;[0 0.902 1] Elige un valor aleatorio para comenzar a moverse.
  (Variables|Default|SetNewDestination (Math|Random|RandomPointinBoundingBox "0, 0,50.000000" (Math|Vector|MakeVector (Variables|Wander|GetMaxBoxExtentX) (Variables|Wander|GetMaxBoxExtentY) (Variables|Wander|GetMaxBoxExtentZ)))))

(event EventTick
  (params (DeltaSeconds :type Float%20%28single-precision%29))
  (Utilities|FlowControl|Sequence
    (:then_0
      (Transformation|SetActorLocationAndRotation (+ (Transformation|GetActorLocation) (* (Transformation|GetActorForwardVector) (Variables|Wander|GetVelocity))) (Math|Interpolation|RInterpTo (Transformation|GetActorRotation) (Math|Rotator|FindLookatRotation (Transformation|GetActorLocation) (Variables|Default|GetNewDestination)) (Utilities|Time|GetWorldDeltaSeconds) 5.0)))
    (:then_1
      ;[1 0 0.1084] Cada 2 segundos eligirá un nuevo lugar al cual dirigirse de manera aleatoria.
      (if (<= (Math|Vector|Distance(Vector) (Transformation|GetActorLocation) (Variables|Default|GetNewDestination)) 1e+02)
        (if (Variables|Wander|GetStopMoving)
          (Variables|Wander|SetVelocity 0.0)
          (else
            (Variables|Default|SetNewDestination (Math|Random|RandomPointinBoundingBox "0, 0,50.000000" (Math|Vector|MakeVector (Variables|Wander|GetMaxBoxExtentX) (Variables|Wander|GetMaxBoxExtentY) (Variables|Wander|GetMaxBoxExtentZ))) :!label _label)
            (Variables|Wander|SetVelocity 1e+01)))
        (else
          (Utilities|FlowControl|Delay (Variables|Wander|GetNewDirectionTime))
          (goto _label))))))

(fn ConstructionScript)